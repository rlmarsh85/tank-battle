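; Player-controlled tank Blueprint that maps input to movement, camera aiming and firing.
; At BeginPlay it hands the barrel and turret to TankAiming and both tracks to TankMovement.
; Drive axes feed TankMovement's forward and turn intents, aim axes rotate the azimuth gimbal and spring arm, and Fire calls TankAiming.
; The construction script sets Projectile_BP as the aiming component's projectile class.
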(event `self.ReceiveBeginPlay`
  (`TankAimingComponent.Initialize` (`self.TankAiming`) (`self.TankBarrel`) (`self.TankTurret1`))
  (`TankMovementComponent.Initialize` (`self.TankMovement`) (`self.LeftTrack1`) (`self.RightTrack1`)))

(event `InputAction|Fire`
  (params (Key :type "Key Structure"))
  (:`Pressed`
    (`TankAimingComponent.Fire` (`self.TankAiming`))))

(event `InputAxis|AimAzimuth`
  (params (AxisValue :type "Float (single-precision)"))
  (`SceneComponent.K2_AddLocalRotation` (`self.AzimuthGimbel`) (`KismetMathLibrary.MakeRotator` 0.0 0.0 (* AxisValue 3.0)) false false))

(event `InputAxis|AimElevation`
  (params (AxisValue :type "Float (single-precision)"))
  (`SceneComponent.K2_AddLocalRotation` (`self.SpringArm`) (`KismetMathLibrary.MakeRotator` 0.0 AxisValue) false false))

(event `InputAxis|Forward`
  (params (AxisValue :type "Float (single-precision)"))
  (`TankMovementComponent.IntendMoveForward` (`self.TankMovement`) AxisValue))

(event `InputAxis|Turn Left`
  (params (AxisValue :type "Float (single-precision)"))
  (`TankMovementComponent.IntendTurnRight` (`self.TankMovement`) AxisValue))

(event `InputAxis|TurnRight`
  (params (AxisValue :type "Float (single-precision)"))
  (`TankMovementComponent.IntendTurnRight` (`self.TankMovement`) AxisValue))

(event `InputAxis|Backward`
  (params (AxisValue :type "Float (single-precision)"))
  (`TankMovementComponent.IntendMoveForward` (`self.TankMovement`) AxisValue))

(fn `UserConstructionScript`
  (locals (NewLocalVar_0 :type "TankAimingComponent Object Reference"))
  (`TankAimingComponent.SetProjectileBPClass` (`self.TankAiming`) "/Game/BT12-TankParts/Projectile_BP.Projectile_BP_C"))